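; Target is an actor with an Ability System component that shows its health on screen, apparently as something to damage.
; On BeginPlay it creates a UI_Health widget attached to itself, adds it to the viewport and triggers an initial health refresh.
; OnHealthChanged reads a float attribute from the Ability System component and passes it to the widget along with the change value as damage.
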(event EventBeginPlay
  (bind _returnvalue (UserInterface|CreateWidget "/Game/UI/UI_Health.UI_Health_C" (Game|GetPlayerController 0) "999" "0.000000,0.000000,30.000000" self))
  (bind _output_get (Variables|Default|SetHealthUI _returnvalue))
  (UserInterface|Viewport|AddtoViewport _output_get 0)
  (Class|STargetActor|OnHealthChanged 0 0.0))

(event EventOnHealthChanged
  (params (K2_Instigator :type Actor%20Object%20Reference) (K2_ChangeValue :type Float%20%28single-precision%29))
  (Default|SetHealthText (Variables|Default|GetHealthUI) (Utilities|Text|ToText(String) (Utilities|String|ToString(Float) (.ReturnValue (Ability|Attribute|GetFloatAttributefromAbilitySystemComponent (Variables|Default|GetAbilitySystemComp) "(AttributeName=\"Health\",Attribute=/Script/Gladiator.SAttributeSetBase:Health,AttributeOwner=/Script/CoreUObject.Class'\"/Script/Gladiator.SAttributeSetBase\"')")))) K2_ChangeValue))

(fn ConstructionScript)