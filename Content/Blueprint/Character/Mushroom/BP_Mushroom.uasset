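; Mushroom character Blueprint whose death triggers the victory screen, apparently serving as an AI-controlled opponent.
; On BeginPlay it offsets its AI controller's UI and creates an attached health widget, which health-change events update from Ability System attributes.
; On death it plays an override animation, removes the health bar, then shows the victory widget after a delay with UI-only input.
; An ability-task delay freezes the death pose via zero time dilation.
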(event EventOnDeath
  (params (K2_Instigator :type Actor%20Object%20Reference))
  (bind _returnvalue (Game|GetPlayerController 0))
  (bind _animationlength (Class|PaperZDAnimInstance|PlayAnimationOverride (Class|PaperZDCharacter|GetAnimInstance) (Variables|Default|GetDeathAnim) "DefaultSlot" 1.0 0.0))
  (GameplayTasks|TaskWaitDelay (Variables|Default|GetAbilitySystemComp) (- _animationlength 0.1)
    (:then
      (Widget|RemovefromParent (Variables|Default|GetHealthUI))
      (Utilities|FlowControl|Delay 2.0)
      (bind _returnvalue_2 (UserInterface|CreateWidget "/Game/UI/UI_Victory.UI_Victory_C" 0 K2_Instigator))
      (UserInterface|Viewport|AddtoViewport _returnvalue_2 0)
      (Input|SetInputModeUIOnly _returnvalue _returnvalue_2 "DoNotLock" true)
      (Variables|/Script/Engine.PlayerController|SetbShowMouseCursor _returnvalue true))
    (:OnFinish
      (Variables|Default|SetCustomTimeDilation 0.0))))

(event EventOnHealthChanged
  (params (K2_Instigator :type Actor%20Object%20Reference) (K2_ChangeValue :type Float%20%28single-precision%29))
  (Default|SetHealth (Variables|Default|GetHealthUI) (.ReturnValue (Ability|Attribute|GetFloatAttributefromAbilitySystemComponent (Variables|Default|GetAbilitySystemComp) "(AttributeName=\"Health\",Attribute=/Script/Gladiator.SAttributeSetBase:Health,AttributeOwner=/Script/CoreUObject.Class'\"/Script/Gladiator.SAttributeSetBase\"')")) K2_ChangeValue))

(event EventBeginPlay
  (bind _asbp_aicontroller (Utilities|Casting|CastToBP_AIController (Pawn|GetController)))
  (Class|SAIController|SetUIWorldOffset _asbp_aicontroller "0.000000,0.000000,90.000000")
  (bind _returnvalue (UserInterface|CreateWidget "/Game/UI/Enemy/UI_Health.UI_Health_C" (Game|GetPlayerController 0) (.ReturnValue (Ability|Attribute|GetFloatAttributefromAbilitySystemComponent (Variables|Default|GetAbilitySystemComp) "(AttributeName=\"MaxHealth\",Attribute=/Script/Gladiator.SAttributeSetBase:MaxHealth,AttributeOwner=/Script/CoreUObject.Class'\"/Script/Gladiator.SAttributeSetBase\"')")) "0.000000,0.000000,80.000000" self))
  (bind _output_get (Variables|Default|SetHealthUI _returnvalue))
  (UserInterface|Viewport|AddtoViewport _output_get 0))

(fn ConstructionScript)